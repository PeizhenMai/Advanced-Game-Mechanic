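; BP_ArchiveLocation is an interactable save point that records a reset location for the player.
; Box overlap toggles a prompt widget and registers or clears the actor as the player character's interaction target.
; The ArchiveLocation event plays a camera shutter sound and stores the Cube's world position as the player's ResetLocation.
; It also moves any BP_ControllCube to an offset beside that Cube and clears the player's IsControllCube flag.
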(event `self.Box.OnComponentBeginOverlap`
  (params (OverlappedComponent :type "PrimitiveComponent Object Reference") (OtherActor :type "Actor Object Reference") (OtherComp :type "PrimitiveComponent Object Reference") (OtherBodyIndex :type Integer) (bFromSweep :type Boolean) (SweepResult :type "HitResult Structure (by ref)"))
  (bind _asbp_player_character (cast `/Game/BluePrints/BP_PlayerCharacter` OtherActor))
  (`SceneComponent.SetHiddenInGame` (`self.Widget`) false false)
  (set `/Game/BluePrints/BP_PlayerCharacter.CanInteract` true _asbp_player_character)
  (set `/Game/BluePrints/BP_PlayerCharacter.Overlap Actor` self _asbp_player_character))

(event `self.Box.OnComponentEndOverlap`
  (params (OverlappedComponent :type "PrimitiveComponent Object Reference") (OtherActor :type "Actor Object Reference") (OtherComp :type "PrimitiveComponent Object Reference") (OtherBodyIndex :type Integer))
  (bind _asbp_player_character (cast `/Game/BluePrints/BP_PlayerCharacter` OtherActor))
  (`SceneComponent.SetHiddenInGame` (`self.Widget`) true false)
  (set `/Game/BluePrints/BP_PlayerCharacter.CanInteract` false _asbp_player_character)
  (set `/Game/BluePrints/BP_PlayerCharacter.Overlap Actor` null _asbp_player_character))

(event `/Game/BluePrints/BI_Interface.ArchiveLocation`
  (bind _returnvalue (`SceneComponent.K2_GetComponentLocation` (`self.Cube`)))
  (`GameplayStatics.PlaySound2D` "/Engine/VREditor/Sounds/UI/Camera_Shutter.Camera_Shutter" 1.0 1.0 0.0 null null)
  (`|ExecutionSequence`
    (:`then_0`
      (bind _asbp_player_character (cast `/Game/BluePrints/BP_PlayerCharacter` (`GameplayStatics.GetPlayerCharacter` 0)))
      (set `/Game/BluePrints/BP_PlayerCharacter.Reset Location` _returnvalue _asbp_player_character))
    (:`then_1`
      (bind _returnvalue_2 (`GameplayStatics.GetActorOfClass` "/Game/BluePrints/BP_ControllCube.BP_ControllCube_C"))
      (`/Engine/EditorBlueprintResources/StandardMacros.IsValid` _returnvalue_2
        (:`Is Valid`
          (`self.K2_SetActorLocation` _returnvalue_2 (`KismetMathLibrary.MakeVector` (+ (.x _returnvalue) 50.0) (.y _returnvalue) (- (.z _returnvalue) 25.0)) false false)
          (set `/Game/BluePrints/BP_PlayerCharacter.isControllCube` false _asbp_player_character))))))

(fn `UserConstructionScript`)