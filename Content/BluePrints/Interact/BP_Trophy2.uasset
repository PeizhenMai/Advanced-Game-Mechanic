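; BP_Trophy2 is an interactable trophy that loads level "03_1" when the player interacts with it.
; Capsule overlap with BP_PlayerCharacter shows or hides a prompt widget and sets the character's CanInteract flag and OverlapActor reference.
; The CharacterInteract event then opens the level by name.
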(event `self.Capsule.OnComponentBeginOverlap`
  (params (OverlappedComponent :type "PrimitiveComponent Object Reference") (OtherActor :type "Actor Object Reference") (OtherComp :type "PrimitiveComponent Object Reference") (OtherBodyIndex :type Integer) (bFromSweep :type Boolean) (SweepResult :type "HitResult Structure (by ref)"))
  (bind _asbp_player_character (cast `/Game/BluePrints/BP_PlayerCharacter` OtherActor))
  (`SceneComponent.SetHiddenInGame` (`self.Widget`) false false)
  (set `/Game/BluePrints/BP_PlayerCharacter.CanInteract` true _asbp_player_character)
  (set `/Game/BluePrints/BP_PlayerCharacter.Overlap Actor` self _asbp_player_character))

(event `self.Capsule.OnComponentEndOverlap`
  (params (OverlappedComponent :type "PrimitiveComponent Object Reference") (OtherActor :type "Actor Object Reference") (OtherComp :type "PrimitiveComponent Object Reference") (OtherBodyIndex :type Integer))
  (bind _asbp_player_character (cast `/Game/BluePrints/BP_PlayerCharacter` OtherActor))
  (`SceneComponent.SetHiddenInGame` (`self.Widget`) true false)
  (set `/Game/BluePrints/BP_PlayerCharacter.CanInteract` false _asbp_player_character)
  (set `/Game/BluePrints/BP_PlayerCharacter.Overlap Actor` null _asbp_player_character))

(event `/Game/BluePrints/BI_Interface.Character Interact`
  (`GameplayStatics.OpenLevel` "03_1"))

(fn `UserConstructionScript`)