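; BP_Door01 is a lockable door whose frame blocks the player while IsLocked is set.
; Every tick it switches the DoorFrame collision between query-and-physics when locked and none when unlocked.
; A Box trigger shows a Widget when the player character enters while the door is locked and hides it on exit if still locked.
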(event `self.ReceiveTick`
  (params (DeltaSeconds :type "Float (single-precision)"))
  (if (`self.IsLocked`)
    (`PrimitiveComponent.SetCollisionEnabled` (`self.DoorFrame`) "QueryAndPhysics")
    (else
      (`PrimitiveComponent.SetCollisionEnabled` (`self.DoorFrame`) "NoCollision"))))

(event `self.Box.OnComponentBeginOverlap`
  (params (OverlappedComponent :type "PrimitiveComponent Object Reference") (OtherActor :type "Actor Object Reference") (OtherComp :type "PrimitiveComponent Object Reference") (OtherBodyIndex :type Integer) (bFromSweep :type Boolean) (SweepResult :type "HitResult Structure (by ref)"))
  (cast `/Game/BluePrints/BP_PlayerCharacter` OtherActor)
  (if (`self.IsLocked`)
    (`SceneComponent.SetHiddenInGame` (`self.Widget`) false false)))

(event `self.Box.OnComponentEndOverlap`
  (params (OverlappedComponent :type "PrimitiveComponent Object Reference") (OtherActor :type "Actor Object Reference") (OtherComp :type "PrimitiveComponent Object Reference") (OtherBodyIndex :type Integer))
  (cast `/Game/BluePrints/BP_PlayerCharacter` OtherActor)
  (if (`self.IsLocked`)
    (`SceneComponent.SetHiddenInGame` (`self.Widget`) true false)))

(fn `UserConstructionScript`)