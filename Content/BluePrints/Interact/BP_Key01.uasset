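; BP_Key01 is an interactable key pickup that unlocks the level's BP_Door01.
; Its Box overlap shows or hides a prompt Widget and registers or clears the key as the BP_PlayerCharacter's interaction target.
; The Key event clears IsLocked on the first BP_Door01 found via GetActorOfClass and plays a 2D sound, without destroying or hiding the key.
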(event `self.Box.OnComponentBeginOverlap`
  (params (OverlappedComponent :type "PrimitiveComponent Object Reference") (OtherActor :type "Actor Object Reference") (OtherComp :type "PrimitiveComponent Object Reference") (OtherBodyIndex :type Integer) (bFromSweep :type Boolean) (SweepResult :type "HitResult Structure (by ref)"))
  (bind _asbp_player_character (cast `/Game/BluePrints/BP_PlayerCharacter` OtherActor))
  (`SceneComponent.SetHiddenInGame` (`self.Widget`) false false)
  (set `/Game/BluePrints/BP_PlayerCharacter.CanInteract` true _asbp_player_character)
  (set `/Game/BluePrints/BP_PlayerCharacter.Overlap Actor` self _asbp_player_character))

(event `self.Box.OnComponentEndOverlap`
  (params (OverlappedComponent :type "PrimitiveComponent Object Reference") (OtherActor :type "Actor Object Reference") (OtherComp :type "PrimitiveComponent Object Reference") (OtherBodyIndex :type Integer))
  (bind _asbp_player_character (cast `/Game/BluePrints/BP_PlayerCharacter` OtherActor))
  (`SceneComponent.SetHiddenInGame` (`self.Widget`) true false)
  (set `/Game/BluePrints/BP_PlayerCharacter.CanInteract` false _asbp_player_character)
  (set `/Game/BluePrints/BP_PlayerCharacter.Overlap Actor` null _asbp_player_character))

(event `/Game/BluePrints/BI_Interface.Key`
  (bind _returnvalue (`GameplayStatics.GetActorOfClass` "/Game/BluePrints/Interact/BP_Door01.BP_Door01_C"))
  (set `/Game/BluePrints/Interact/BP_Door01.IsLocked` false _returnvalue)
  (`GameplayStatics.PlaySound2D` "/Engine/VREditor/Sounds/UI/Object_Snaps_To_Another_Actor.Object_Snaps_To_Another_Actor" 1.0 1.0 0.0 null null))

(fn `UserConstructionScript`)