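; BP_ControllCube is a cube actor that the player character can take control of and that can replay a series of movements.
; Every Tick it reads IsControllCube from BP_PlayerCharacter, disabling physics simulation while controlled and enabling it otherwise.
; Cube Replay consumes BlockMovementDeltas front to back as swept local offsets, clearing its timer when the array empties.
; Neither the recording of deltas nor the timer start happens in this Blueprint.
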(event `self.ReceiveTick`
  (params (DeltaSeconds :type "Float (single-precision)"))
  (bind _asbp_player_character (cast `/Game/BluePrints/BP_PlayerCharacter` (`GameplayStatics.GetPlayerCharacter` 0)))
  (if (`/Game/BluePrints/BP_PlayerCharacter.isControllCube` _asbp_player_character)
    (`PrimitiveComponent.SetSimulatePhysics` (`self.Cube`) false)
    (else
      (`PrimitiveComponent.SetSimulatePhysics` (`self.Cube`) true))))

(fn `Cube Replay`
  (bind _block_movementdeltas (`self.Block MovementDeltas`))
  (if (== (`KismetArrayLibrary.Array_Length` _block_movementdeltas) 0)
    (`KismetSystemLibrary.K2_ClearTimer` null "Cube Replay")
    (else
      (`self.K2_AddActorLocalOffset` (`|GetArrayItem` _block_movementdeltas) true)
      (`KismetArrayLibrary.Array_Remove` (`self.Block MovementDeltas`)))))

(fn `UserConstructionScript`)